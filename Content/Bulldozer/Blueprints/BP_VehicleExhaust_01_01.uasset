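; Scene component for vehicle exhaust in the Bulldozer game that drives a particle effect from an intensity value.
; On BeginPlay it spawns the particle template attached to itself and starts it at zero intensity.
; SetIntensity samples the RPMToSpawn and RPMToVelocity curves, writing the results to the emitter's exhaust intensity and vertical velocity parameters.
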(event `self.ReceiveBeginPlay`
  (bind _returnvalue (`GameplayStatics.SpawnEmitterAttached` (`self.ParticleTemplate`) self "None" (0.0 0.0 0.0) (struct) (1.0 1.0 1.0) "KeepRelativeOffset" true "AutoRelease"))
  (set `self.CurrentExhaust` _returnvalue)
  (`self.SetIntensity` 0.0))

(fn `SetIntensity`
  (params (Intensity :type "Float (double-precision)"))
  (`ParticleSystemComponent.SetFloatParameter` (`self.CurrentExhaust`) "ExhaustIntensity" (`CurveFloat.GetFloatValue` (`self.RPM to Spawn`) Intensity))
  (`ParticleSystemComponent.SetVectorParameter` (`self.CurrentExhaust`) "Velocity" (`KismetMathLibrary.MakeVector` 0.0 0.0 (`CurveFloat.GetFloatValue` (`self.RPM to Velocity`) Intensity))))