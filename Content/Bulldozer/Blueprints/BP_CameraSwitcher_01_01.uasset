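; Camera switcher in the Bulldozer folder that activates one camera from a supplied list, by index or as first, last, next or previous.
; SetSpringArms caches each arm's initial rotation and length, which activation restores for every index except 1.
; Activation deactivates all other cameras and tracks the current spring arm; indices past the end wrap to zero, but negative ones are unhandled.
; A spring arm zoom value is stored but unused here.
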(fn `ActivateByNumber`
  (params (Index :type Integer))
  (bind _cameras (`self.Cameras`))
  (bind _returnvalue (`KismetArrayLibrary.Array_Length` _cameras))
  (bind _returnvalue_2 (`KismetMathLibrary.SelectInt` 0 Index (> Index (- _returnvalue 1))))
  (if (> _returnvalue 0)
    (bind _succeded (`self.ActivateCamera` (`|GetArrayItem` _cameras _returnvalue_2) _returnvalue_2))
    (if _succeded
      (set `self.CurrentCamera` _returnvalue_2))))

(fn `ActivateCamera`
  (params (Camera :type "CameraComponent Object Reference") (index :type Integer))
  (returns (Succeded :type Boolean))
  (bind _output (`|GetArrayItem` (`self.SpringArms`) index))
  (`/Engine/EditorBlueprintResources/StandardMacros.IsValid` Camera
    (:`Is Valid`
      (for _array_element (`self.Cameras`)
        (`self.SetActive` _array_element false true))
      (`self.SetActive` Camera true false)
      (set `self.CurrentSpringArm` _output)
      (if (!= index 1)
        (`SceneComponent.K2_SetRelativeRotation` _output (`|GetArrayItem` (`self.SpringArmRotation`) index) false false)
        (set `SpringArmComponent.TargetArmLength` (`|GetArrayItem` (`self.SpringArmLength`) index) (`self.CurrentSpringArm`))
        (return true)
        (else
          (return true))))
    (:`Is Not Valid`
      (return false))))

(fn `ActivateFirst`
  (`self.ActivateByNumber` 0))

(fn `ActivateLast`
  (`self.ActivateByNumber` (- (`KismetArrayLibrary.Array_Length` (`self.Cameras`)) 1)))

(fn `ActivateNext`
  (`self.ActivateByNumber` (+ (`self.CurrentCamera`) 1)))

(fn `ActivatePrevious`
  (`self.ActivateByNumber` (- (`self.CurrentCamera`) 1)))

(fn `SetCameras`
  (params (Cameras :type "Array of CameraComponent Object Reference"))
  (set `self.Cameras` Cameras))

(fn `SetSpringArms`
  (params (SpringArms :type "Array of SpringArmComponent Object Reference"))
  (`|ExecutionSequence`
    (:`then_0`
      (set `self.SpringArms` SpringArms))
    (:`then_1`
      (for (_array_element _array_index) SpringArms
        (`KismetArrayLibrary.Array_Set` (`self.SpringArmRotation`) _array_index (`SceneComponent.RelativeRotation` _array_element) true)
        (`KismetArrayLibrary.Array_Set` (`self.SpringArmLength`) _array_index (`SpringArmComponent.TargetArmLength` _array_element) true)))))

(fn `SetSpringArmZoom`
  (params (Zoom :type "Array of Vector Structure"))
  (set `self.SpringArmZoom` Zoom))