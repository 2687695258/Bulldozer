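; Wheel effect component for BP_Vehicle that switches surface particles and builds up mud as the vehicle drives.
; At BeginPlay it attaches deactivated emitters to the owner's mesh and puts a dynamic mud material on tagged meshes.
; While moving, a downward trace's physical material selects the mud, water or default emitter.
; Mud accumulates on mud and fades elsewhere, feeding that material and a per-wheel parameter in a Material Parameter Collection.
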(event `self.ReceiveBeginPlay`
  (bind _asbp_vehicle (cast `/Game/Bulldozer/Blueprints/BP_Vehicle` (`self.GetOwner`)))
  (set `self.Owner` _asbp_vehicle)
  (for _array_element (`self.Particles`)
    (bind _returnvalue (`GameplayStatics.SpawnEmitterAttached` _array_element (`WheeledVehiclePawn.Mesh` (`self.Owner`)) "None" (`self.RelativeLocation`) (struct) (1.0 1.0 1.0) "KeepRelativeOffset" false))
    (`KismetArrayLibrary.Array_Add` (`self.SpawnedParticles`) _returnvalue))
  (for _array_element_2 (`self.SpawnedParticles`)
    (`self.Deactivate` _array_element_2)
    (`self.SetAutoActivate` _array_element_2 false))
  (bind _returnvalue_2 (`KismetMaterialLibrary.CreateDynamicMaterialInstance` (`self.MudMaterial`)))
  (set `self.MudMID` _returnvalue_2)
  (for _array_element_3 (`Actor.GetComponentsByTag` (`self.Owner`) "/Script/Engine.ActorComponent" (`self.MudMeshTag`))
    (bind `_as静态网格体组件` (cast `StaticMeshComponent` _array_element_3))
    (`PrimitiveComponent.SetMaterial` `_as静态网格体组件` 0 (`self.MudMID`))))

(event `self.ReceiveTick`
  (params (DeltaSeconds :type "Float (single-precision)"))
  (bind _returnvalue (`self.K2_GetComponentLocation`))
  (bind _spawnedparticles (`self.SpawnedParticles`))
  (bind _mudvalue (`self.MudValue`))
  (bind _mudvalue_2 (`self.MudValue`))
  (bind _returnvalue_2 (/ (`self.MudValue`) 5.0))
  (bind _output (`|GetArrayItem` _spawnedparticles 1))
  (bind _output_2 (`|GetArrayItem` _spawnedparticles 2))
  (if (> (`KismetMathLibrary.Abs` (`ChaosVehicleMovementComponent.GetForwardSpeed` (`WheeledVehiclePawn.VehicleMovementComponent` (`self.Owner`)))) 50.0)
    (bind (_outhit _returnvalue_3) (`KismetSystemLibrary.LineTraceSingle` (+ _returnvalue (0.0 0.0 40.0)) (+ _returnvalue (0.0 0.0 -20.0)) "TraceTypeQuery1" true (`|MakeArray` (`self.Owner`) :!type "Actor Object Reference") "None" true (struct :`R` 1.0 :`A` 1.0) (struct :`G` 1.0 :`A` 1.0) 20.0))
    (if _returnvalue_3
      (bind (_bblockinghit _binitialoverlap _time _distance _location _impactpoint _normal _impactnormal _physmat) (`GameplayStatics.BreakHitResult` _outhit))
      (if (== _physmat "/Game/Bulldozer/Material/pm_Mud_01_01.pm_Mud_01_01")
        (`self.SetActive` _output true false)
        (`self.Deactivate` _output_2)
        (`self.Deactivate` (`|GetArrayItem` _spawnedparticles))
        (if (< _mudvalue 5.0)
          (set `self.MudValue` (+ _mudvalue DeltaSeconds))
          (`KismetMaterialLibrary.SetScalarParameterValue` "/Game/Bulldozer/Material/mpc_VehiclesParam_01_01.mpc_VehiclesParam_01_01" (`KismetStringLibrary.Conv_StringToName` (`|GetEnumeratorNameAsString` (`self.Wheel`))) _returnvalue_2 :!label _label)
          (`MaterialInstanceDynamic.SetScalarParameterValue` (`self.MudMID`) "Mud" _returnvalue_2))
        (else
          (if (== _physmat "/Game/Bulldozer/Material/pm_Water_01_01.pm_Water_01_01")
            (`self.SetActive` _output_2 true false)
            (`self.Deactivate` _output)
            (`self.Deactivate` (`|GetArrayItem` _spawnedparticles))
            (else
              (`self.SetActive` (`|GetArrayItem` _spawnedparticles) true false)
              (`self.Deactivate` _output)
              (`self.Deactivate` _output_2)))
          (if (> _mudvalue_2 0.0)
            (set `self.MudValue` (- _mudvalue_2 DeltaSeconds))
            (goto _label))))
      (else
        (for _array_element (`self.SpawnedParticles`) :!label _label_2
          (`self.Deactivate` _array_element))))
    (else
      (goto _label_2))))